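; Base Blueprint for a player weapon drawn as a Paper2D flipbook, with a scene capture that renders only that flipbook.
; Initialization calls SetFlipbook with no flipbook specified and hides the component in game.
; The bobbing event plays or stops the GunBob sequence player based on movement.
; The weapon's starting position is cached, but the interpolation back to it is disconnected and never runs.
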(event `self.ReceiveBeginPlay`
  (`SceneCaptureComponent.ShowOnlyComponent` (`self.SceneCaptureComponent2D`) (`self.Weapon Flipbook`))
  (set `self.Weapon Pos` (`SceneComponent.RelativeLocation` (`self.Weapon Flipbook`))))

(event `/Game/Blueprints/IPlayerInterface.Initialize Weapon`
  (bind _weapon_flipbook (`self.Weapon Flipbook`))
  (`PaperFlipbookComponent.SetFlipbook` _weapon_flipbook null)
  (`SceneComponent.SetHiddenInGame` _weapon_flipbook true false))

(event `WEapon Bobbing`
  (params (isMoving :type Boolean) (DeltaTime :type "Float (double-precision)"))
  (bind _sequenceplayer (`ActorSequenceComponent.SequencePlayer` (`self.Gun Bob`)))
  (if isMoving
    (`MovieSceneSequencePlayer.Play` _sequenceplayer)
    (else
      (`MovieSceneSequencePlayer.Stop` _sequenceplayer))))

(fn `UserConstructionScript`)